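; Fast enemy turret that turns toward a seen player character and fires BP_EnemyBullet after a FireRate delay.
; BeginPlay loads FireRate and Hp from the FastTurret row of DT_Enemy; Hp is not used afterwards.
; Overlaps briefly set EngageColor red on a dynamic material and print a debug hit, without applying damage.
; The mesh is assigned EnemyHPStatus rather than the created dynamic instance.
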(event OnSeePawn(PawnSensing)
  (params (Pawn :type Pawn%20Object%20Reference))
  (bind _asue4_project_vjm5ahcharacter (Utilities|Casting|CastToUE4_Project_VJM5AHCharacter Pawn)
    (:then
      _)
    (:CastFailed
      _))
  (Transformation|SetActorRotation (Math|Rotator|FindLookatRotation (Transformation|GetActorLocation) (Transformation|GetActorLocation _asue4_project_vjm5ahcharacter)))
  (Utilities|FlowControl|Delay (Variables|Default|GetfireRate))
  (Game|SpawnActorfromClass "/Game/Blueprints/Enemy/BP_EnemyBullet.BP_EnemyBullet_C" (Transformation|GetWorldTransform (Variables|Default|GetBulletSpawnPosition)) "Undefined" 0 0))

(event EventBeginPlay
  (bind _returnvalue (Rendering|Material|CreateDynamicMaterialInstance "/Game/Materials/DynamicMaterials/EnemyHPStatus.EnemyHPStatus" "None" "None" :!class /Script/Engine.KismetMaterialLibrary))
  (Variables|Default|SetDynMaterial _returnvalue)
  (Rendering|Material|SetMaterial (Variables|Default|GetStaticMesh) 0 "/Game/Materials/DynamicMaterials/EnemyHPStatus.EnemyHPStatus")
  (bind _returnvalue_2 (Utilities|GetDataTableRow "/Game/DataTable/DTEnemy/DT_Enemy.DT_Enemy" "FastTurret")
    (:then
      (Variables|Default|SetfireRate (.FireRate (Utilities|Struct|BreakStructEnemy _returnvalue_2)))
      (Variables|Default|Sethp (.Life (Utilities|Struct|BreakStructEnemy _returnvalue_2))))))

(event Collision|EventActorBeginOverlap
  (params (OtherActor :type Actor%20Object%20Reference))
  (bind _dynmaterial (Variables|Default|GetDynMaterial))
  (Rendering|Material|SetVectorParameterValue _dynmaterial "EngageColor" "(R=1.000000,G=0.000000,B=0.000000,A=1.000000)" :!class /Script/Engine.MaterialInstanceDynamic)
  (Utilities|FlowControl|Delay 0.3)
  (Rendering|Material|SetVectorParameterValue _dynmaterial "EngageColor" "(R=0.000000,G=0.000000,B=0.000000,A=1.000000)" :!class /Script/Engine.MaterialInstanceDynamic)
  (Development|PrintString "HIT"))

(event EventTick
  (params (DeltaSeconds :type Float%20%28single-precision%29)))

(fn ConstructionScript)